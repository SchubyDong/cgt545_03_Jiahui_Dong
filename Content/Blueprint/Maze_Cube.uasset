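; Maze_Cube is a musical memory puzzle that removes a fog actor when the player reproduces a note sequence.
; Entering the Box trigger clears the answer and plays a hardcoded, timed demo tune, highlighting each cube in blue.
; Player overlaps on the four cube colliders play notes, recolor cubes and append digits to a string.
; Tick compares that string to Sequence, destroying the fog and starting music on a match.
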(event `self.ReceiveTick`
  (params (DeltaSeconds :type "Float (single-precision)"))
  (if (== (`self.Sequence`) (`self.User_Answer`))
    (bind _the_fog (`self.The fog`)
      (:`then`
        (`self.K2_DestroyActor` _the_fog)
        (`/Engine/EditorBlueprintResources/StandardMacros.DoOnce` false :!label _label
          (:`Completed`
            (`GameplayStatics.PlaySound2D` "/Game/Sound/y2mate_is_-_Child_of_Light_OST_13_Down_to_a_Dusty_Plain-aDf5w4Stk6A-192k-1701646389.y2mate_is_-_Child_of_Light_OST_13_Down_to_a_Dusty_Plain-aDf5w4Stk6A-192k-1701646389" 1.0 1.0 0.0 null null)
            (`KismetSystemLibrary.Delay` 180.0)
            (goto _label :!via `Reset`))))
      (:`else`))))

(event `self.2_Collision.OnComponentBeginOverlap`
  (params (OverlappedComponent :type "PrimitiveComponent Object Reference") (OtherActor :type "Actor Object Reference") (OtherComp :type "PrimitiveComponent Object Reference") (OtherBodyIndex :type Integer) (bFromSweep :type Boolean) (SweepResult :type "HitResult Structure (by ref)"))
  (cast `/Game/FirstPerson/Blueprints/BP_FirstPersonCharacter` OtherActor)
  (`GameplayStatics.PlaySound2D` "/Game/Sound/2.2" 1.0 1.0 0.0 null null)
  (set `self.User_Answer` (`KismetStringLibrary.Concat_StrStr` (`self.User_Answer`) "2"))
  (`self.Change the cube color` (`self.2`))
  (`KismetSystemLibrary.PrintString` (`self.User_Answer`) :!label _label_2))

(event `self.3_Collision.OnComponentBeginOverlap`
  (params (OverlappedComponent :type "PrimitiveComponent Object Reference") (OtherActor :type "Actor Object Reference") (OtherComp :type "PrimitiveComponent Object Reference") (OtherBodyIndex :type Integer) (bFromSweep :type Boolean) (SweepResult :type "HitResult Structure (by ref)"))
  (cast `/Game/FirstPerson/Blueprints/BP_FirstPersonCharacter` OtherActor)
  (`GameplayStatics.PlaySound2D` "/Game/Sound/3.3" 1.0 1.0 0.0 null null)
  (set `self.User_Answer` (`KismetStringLibrary.Concat_StrStr` (`self.User_Answer`) "3"))
  (`self.Change the cube color` (`self.3`))
  (goto _label_2))

(event `self.4_Collision.OnComponentBeginOverlap`
  (params (OverlappedComponent :type "PrimitiveComponent Object Reference") (OtherActor :type "Actor Object Reference") (OtherComp :type "PrimitiveComponent Object Reference") (OtherBodyIndex :type Integer) (bFromSweep :type Boolean) (SweepResult :type "HitResult Structure (by ref)"))
  (cast `/Game/FirstPerson/Blueprints/BP_FirstPersonCharacter` OtherActor)
  (`GameplayStatics.PlaySound2D` "/Game/Sound/4.4" 1.0 1.0 0.0 null null)
  (set `self.User_Answer` (`KismetStringLibrary.Concat_StrStr` (`self.User_Answer`) "4"))
  (`self.Change the cube color` (`self.4`))
  (goto _label_2))

(event `self.5_Collision.OnComponentBeginOverlap`
  (params (OverlappedComponent :type "PrimitiveComponent Object Reference") (OtherActor :type "Actor Object Reference") (OtherComp :type "PrimitiveComponent Object Reference") (OtherBodyIndex :type Integer) (bFromSweep :type Boolean) (SweepResult :type "HitResult Structure (by ref)"))
  (cast `/Game/FirstPerson/Blueprints/BP_FirstPersonCharacter` OtherActor)
  (`GameplayStatics.PlaySound2D` "/Game/Sound/5.5" 1.0 1.0 0.0 null null)
  (set `self.User_Answer` (`KismetStringLibrary.Concat_StrStr` (`self.User_Answer`) "5"))
  (`self.Change the cube color` (`self.5`))
  (goto _label_2))

(event `self.Box.OnComponentBeginOverlap`
  (params (OverlappedComponent :type "PrimitiveComponent Object Reference") (OtherActor :type "Actor Object Reference") (OtherComp :type "PrimitiveComponent Object Reference") (OtherBodyIndex :type Integer) (bFromSweep :type Boolean) (SweepResult :type "HitResult Structure (by ref)"))
  (cast `/Game/FirstPerson/Blueprints/BP_FirstPersonCharacter` OtherActor)
  (`/Engine/EditorBlueprintResources/StandardMacros.DoOnce` false :!label _label_3
    (:`Completed`
      (set `self.User_Answer` "")
      (`self.Change the cube color` (`self.2`))
      (`GameplayStatics.PlaySound2D` "/Game/Sound/2.2" 1.0 1.0 0.0 null null)
      (`KismetSystemLibrary.Delay` 0.5)
      (`self.Change the cube color` (`self.3`))
      (`GameplayStatics.PlaySound2D` "/Game/Sound/3.3" 1.0 1.0 0.0 null null)
      (`KismetSystemLibrary.Delay` 0.5)
      (`self.Change the cube color` (`self.4`))
      (`GameplayStatics.PlaySound2D` "/Game/Sound/4.4" 1.0 1.0 0.0 null null)
      (`KismetSystemLibrary.Delay` 0.5)
      (`self.Change the cube color` (`self.2`))
      (`GameplayStatics.PlaySound2D` "/Game/Sound/2.2" 1.0 1.0 0.0 null null)
      (`KismetSystemLibrary.Delay` 0.5)
      (`self.Change the cube color` (`self.3`))
      (`GameplayStatics.PlaySound2D` "/Game/Sound/3.3" 1.0 1.0 0.0 null null)
      (`KismetSystemLibrary.Delay` 0.5)
      (`self.Change the cube color` (`self.5`))
      (`GameplayStatics.PlaySound2D` "/Game/Sound/5.5" 1.0 1.0 0.0 null null)
      (`KismetSystemLibrary.Delay` 0.5)
      (`self.Change the cube color` (`self.4`))
      (`GameplayStatics.PlaySound2D` "/Game/Sound/4.4" 1.0 1.0 0.0 null null)
      (`KismetSystemLibrary.Delay` 0.5)
      (`self.Change the cube color` (`self.3`))
      (`GameplayStatics.PlaySound2D` "/Game/Sound/3.3" 1.0 1.0 0.0 null null)
      (`KismetSystemLibrary.Delay` 0.5)
      (`self.Change the cube color` (`self.2`))
      (`GameplayStatics.PlaySound2D` "/Game/Sound/2.2" 1.0 1.0 0.0 null null)
      (`KismetSystemLibrary.Delay` 0.5))))

(event `self.Box.OnComponentEndOverlap`
  (params (OverlappedComponent :type "PrimitiveComponent Object Reference") (OtherActor :type "Actor Object Reference") (OtherComp :type "PrimitiveComponent Object Reference") (OtherBodyIndex :type Integer))
  (cast `/Game/FirstPerson/Blueprints/BP_FirstPersonCharacter` OtherActor)
  (goto _label_3 :!via `Reset`))

(fn `Change the cube color`
  (params (`Target Cube` :type "StaticMeshComponent Object Reference"))
  (`PrimitiveComponent.SetMaterial` (`self.2`) 0 "/Game/PortalsAR/DemoCharacter/FirstPerson/Meshes/BaseMaterial.BaseMaterial")
  (`PrimitiveComponent.SetMaterial` (`self.3`) 0 "/Game/PortalsAR/DemoCharacter/FirstPerson/Meshes/BaseMaterial.BaseMaterial")
  (`PrimitiveComponent.SetMaterial` (`self.4`) 0 "/Game/PortalsAR/DemoCharacter/FirstPerson/Meshes/BaseMaterial.BaseMaterial")
  (`PrimitiveComponent.SetMaterial` (`self.5`) 0 "/Game/PortalsAR/DemoCharacter/FirstPerson/Meshes/BaseMaterial.BaseMaterial")
  (`PrimitiveComponent.SetMaterial` `Target Cube` 0 "/Game/LevelPrototyping/Materials/MI_Solid_Blue.MI_Solid_Blue"))

(fn `UserConstructionScript`)