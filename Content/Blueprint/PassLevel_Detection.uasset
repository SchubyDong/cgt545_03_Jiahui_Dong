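; PassLevel_Detection is a trigger actor that marks the level as won when the first-person character enters its box.
; The box overlap sets IsWin on the character.
; While that flag is true, Tick lowers the referenced fog's density and the character's post-process blend weight by a fixed step each frame, with no delta-time scaling or explicit clamp.
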(event `self.ReceiveTick`
  (params (DeltaSeconds :type "Float (single-precision)"))
  (bind _asbp_first_person_character (cast `/Game/FirstPerson/Blueprints/BP_FirstPersonCharacter` (`GameplayStatics.GetPlayerPawn` 0) :!pure true))
  (bind _component (`ExponentialHeightFog.Component` (`self.Fog`)))
  (bind _postprocess (`/Game/FirstPerson/Blueprints/BP_FirstPersonCharacter.PostProcess` _asbp_first_person_character))
  (if (`/Game/FirstPerson/Blueprints/BP_FirstPersonCharacter.Is_Win` _asbp_first_person_character)
    (`ExponentialHeightFogComponent.SetFogDensity` _component (- (`ExponentialHeightFogComponent.FogDensity` _component) 0.05))
    (set `PostProcessComponent.BlendWeight` (- (`PostProcessComponent.BlendWeight` _postprocess) 0.05) _postprocess)))

(event `self.Box.OnComponentBeginOverlap`
  (params (OverlappedComponent :type "PrimitiveComponent Object Reference") (OtherActor :type "Actor Object Reference") (OtherComp :type "PrimitiveComponent Object Reference") (OtherBodyIndex :type Integer) (bFromSweep :type Boolean) (SweepResult :type "HitResult Structure (by ref)"))
  (bind _asbp_first_person_character (cast `/Game/FirstPerson/Blueprints/BP_FirstPersonCharacter` OtherActor))
  (set `/Game/FirstPerson/Blueprints/BP_FirstPersonCharacter.Is_Win` true _asbp_first_person_character))

(fn `UserConstructionScript`)